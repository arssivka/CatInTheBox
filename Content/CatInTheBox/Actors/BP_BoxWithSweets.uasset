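; BP_BoxWithSweets is a spawner box that keeps supplying random sweets at its spawn point.
; A looping timer calls SpawnSweets, which spawns an actor from the SweetClass array at SpawnPoint.
; SpawnCollider tracks overlapping BP_Sweets in a set, pausing the timer while any are inside and resuming it when the set empties.
; The validity check and the spawn roll separate random indices, so they can pick different classes.
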(event `self.ReceiveBeginPlay`
  (bind _returnvalue (`KismetSystemLibrary.K2_SetTimer` null "SpawnSweets" 1.0 true))
  (set `self.SweetSpawnTimer` _returnvalue))

(event `self.SpawnCollider.OnComponentBeginOverlap`
  (params (OverlappedComponent :type "PrimitiveComponent Object Reference") (OtherActor :type "Actor Object Reference") (OtherComp :type "PrimitiveComponent Object Reference") (OtherBodyIndex :type Integer) (bFromSweep :type Boolean) (SweepResult :type "HitResult Structure (by ref)"))
  (bind _asbp_sweets (cast `/Game/CatInTheBox/Actors/BP_Sweets` OtherActor))
  (`BlueprintSetLibrary.Set_Add` (`self.ActorsInTheBox`) _asbp_sweets)
  (`KismetSystemLibrary.K2_PauseTimerHandle` (`self.SweetSpawnTimer`)))

(event `self.SpawnCollider.OnComponentEndOverlap`
  (params (OverlappedComponent :type "PrimitiveComponent Object Reference") (OtherActor :type "Actor Object Reference") (OtherComp :type "PrimitiveComponent Object Reference") (OtherBodyIndex :type Integer))
  (bind _asbp_sweets (cast `/Game/CatInTheBox/Actors/BP_Sweets` OtherActor))
  (`BlueprintSetLibrary.Set_Remove` (`self.ActorsInTheBox`) _asbp_sweets)
  (if (`BlueprintSetLibrary.Set_IsEmpty` (`self.ActorsInTheBox`))
    (`KismetSystemLibrary.K2_UnPauseTimerHandle` (`self.SweetSpawnTimer`))))

(fn `SpawnSweets`
  (bind _sweetclass (`self.SweetClass`))
  (bind _output (`|ConvertAsset` (`|GetArrayItem` _sweetclass (`KismetMathLibrary.RandomInteger` (`KismetArrayLibrary.Array_Length` _sweetclass)))))
  (if (`KismetSystemLibrary.IsValidClass` _output)
    (`|SpawnActorFromClass` _output (`SceneComponent.K2_GetComponentToWorld` (`self.SpawnPoint`)) "Undefined" "MultiplyWithRoot" null null)))

(fn `UserConstructionScript`)
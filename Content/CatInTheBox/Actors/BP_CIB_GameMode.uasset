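; Game mode for CatInTheBox that keeps spawning cats around the player.
; On BeginPlay it starts a looping two-second timer, with a randomly varied initial delay, that calls SpawnCat.
; If the player pawn is valid, SpawnCat spawns an actor at a random angle and distance between MinRadius and MaxRadius around it, lowered by a fixed offset, with yaw from a look-at rotation toward the player.
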(event `self.ReceiveBeginPlay`
  (`KismetSystemLibrary.K2_SetTimer` null "SpawnCat" 2.0 true false 0.0 5.0))

(fn `SpawnCat`
  (bind _returnvalue (`GameplayStatics.GetPlayerPawn` 0))
  (bind _returnvalue_2 (`self.K2_GetActorLocation` _returnvalue))
  (bind _returnvalue_3 (+ _returnvalue_2 (* (`KismetMathLibrary.Conv_RotatorToVector` (`KismetMathLibrary.RotatorFromAxisAndAngle` (0.0 0.0 1.0) (`KismetMathLibrary.RandomFloatInRange` 0.0 360.0))) (`KismetMathLibrary.RandomFloatInRange` (`self.MinRadius`) (`self.MaxRadius`)))))
  (bind (_returnvalue_roll _returnvalue_pitch _returnvalue_yaw) (`KismetMathLibrary.BreakRotator` (`KismetMathLibrary.FindLookAtRotation` _returnvalue_3 _returnvalue_2)))
  (`/Engine/EditorBlueprintResources/StandardMacros.IsValid` _returnvalue
    (:`Is Valid`
      (`|SpawnActorFromClass` "/Game/CatInTheBox/Actors/BP_CatInTheBox.BP_CatInTheBox_C" (`KismetMathLibrary.MakeTransform` (- _returnvalue_3 (0.0 0.0 100.0)) (`KismetMathLibrary.MakeRotator` 0.0 0.0 _returnvalue_yaw)) "Undefined" "MultiplyWithRoot" null null))))

(fn `UserConstructionScript`)
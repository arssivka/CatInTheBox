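; BP_CIB_HUD is the Cat In The Box HUD that creates the main UI and shows a tutorial when play begins.
; On BeginPlay it adds BP_MainUI to the viewport, then pushes WBP_TutorialWidget onto that UI's dialog stack.
; It binds the tutorial's Got It event, which marks the tutorial as accepted and pops the widget off the stack.
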(event `self.ReceiveBeginPlay`
  (bind _returnvalue (`|CreateWidget` "/Game/CatInTheBox/UI/BP_MainUI.BP_MainUI_C" (`GameplayStatics.GetPlayerController` 0)))
  (set `self.MainUI` _returnvalue)
  (`UserWidget.AddToViewport` _returnvalue 0)
  (bind _returnvalue_2 (`/Game/CatInTheBox/UI/BP_MainUI.PushDialogStack` _returnvalue "/Game/CatInTheBox/UI/WBP_TutorialWidget.WBP_TutorialWidget_C"))
  (bind _aswbp_tutorial_widget (cast `/Game/CatInTheBox/UI/WBP_TutorialWidget` _returnvalue_2))
  (bind _output_get (set `self.Tutorial Widget` _aswbp_tutorial_widget))
  (add `/Game/CatInTheBox/UI/WBP_TutorialWidget.GotItEvent` _output_get (delegate `GotIt`)))

(event `GotIt`
  (set `self.TutorialAccepted` true)
  (`/Game/CatInTheBox/UI/BP_MainUI.PopDialogStack` (`self.MainUI`) (`self.Tutorial Widget`)))

(fn `UserConstructionScript`)
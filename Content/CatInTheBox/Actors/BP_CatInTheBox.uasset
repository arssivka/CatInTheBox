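; BP_CatInTheBox is a cat-in-a-box actor that appears, bobs up and waits to be fed sweets.
; On BeginPlay, one timeline drives the cat's vertical jump while another scales cloud, box and cat for the spawn, then marks the cat ready.
; A BP_Sweets overlap while ready plays a happy meow and reverses the spawn timeline, whose Finished branch then destroys the actor.
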(event `self.ReceiveBeginPlay`
  (set `self.InitialCatLocation` (`SceneComponent.RelativeLocation` (`self.SM_Cat`)))
  (`|ExecutionSequence`
    (:`then_0`
      (bind (_direction _jumpheight) (`Timeline|CatJumping`)
        (:`Update`
          (`SceneComponent.K2_SetRelativeLocation` (`self.SM_Cat`) (+ (* (`KismetMathLibrary.Vector_Up`) (* _jumpheight (`self.JumpHeight`))) (`self.InitialCatLocation`)) false false))))
    (:`then_1`
      (bind (_direction_2 _cloudscale _boxscale _catscale) (`Timeline|CatSpawning` :!label _label)
        (:`Update`
          (`|ExecutionSequence`
            (:`then_0`
              (`SceneComponent.SetRelativeScale3D` (`self.SM_Cloud`) (`KismetMathLibrary.Conv_DoubleToVector` (* _cloudscale (`self.CloudScale`)))))
            (:`then_1`
              (`SceneComponent.SetRelativeScale3D` (`self.SM_Box`) (`KismetMathLibrary.Conv_DoubleToVector` _boxscale)))
            (:`then_2`
              (`SceneComponent.SetRelativeScale3D` (`self.SM_Cat`) (`KismetMathLibrary.Conv_DoubleToVector` _catscale)))))
        (:`Finished`
          (set `self.CatReady` true)
          (if (`self.ReadyToDestroy`)
            (`self.K2_DestroyActor`)))))))

(event `self.SweetsConsumerCollision.OnComponentBeginOverlap`
  (params (OverlappedComponent :type "PrimitiveComponent Object Reference") (OtherActor :type "Actor Object Reference") (OtherComp :type "PrimitiveComponent Object Reference") (OtherBodyIndex :type Integer) (bFromSweep :type Boolean) (SweepResult :type "HitResult Structure (by ref)"))
  (if (`self.CatReady`)
    (cast `/Game/CatInTheBox/Actors/BP_Sweets` OtherActor)
    (`GameplayStatics.SpawnSoundAttached` "/Game/CatInTheBox/Audio/MS_HappyMeow.MS_HappyMeow" (`self.SM_Cat`) "None" (0.0 0.0 0.0) (struct) "KeepRelativeOffset" false 1.0 1.0 0.0 null null)
    (set `self.ReadyToDestroy` true)
    (set `self.CatReady` false)
    (goto _label :!via `ReverseFromEnd`)))

(fn `UserConstructionScript`)